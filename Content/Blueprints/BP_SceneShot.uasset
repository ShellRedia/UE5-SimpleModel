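; BP_SceneShot is an actor that tracks facial keypoint locations on a MetaHuman in the level.
; On BeginPlay it finds the first actor of the class selected by MetaHumanIndex, casts it to BP_Aoi and caches its Face component.
; Each Tick, it samples that component's socket location for every name in KeypointsNames into the index-matched KeypointsLoc array.
; The cast ties it to BP_Aoi, so other MetaHuman classes leave the face reference unset.
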(event EventBeginPlay
  (bind _outactors (Actor|GetAllActorsOfClass (Utilities|Array|Get(acopy) (Variables|Default|GetMetaHumanClasses) (Variables|Default|GetMetaHumanIndex))))
  (bind _output_get (Variables|Default|SetMetaHumanRef (Utilities|Array|Get(acopy) _outactors)))
  (bind _asbp_aoi (Utilities|Casting|CastToBP_Aoi _output_get))
  (Variables|Default|SetFaceSkeletal (Variables|/Game/MetaHumans/Aoi/BP_Aoi.BP_Aoi_C|GetFace _asbp_aoi)))

(event Collision|EventActorBeginOverlap
  (params (OtherActor :type Actor%20Object%20Reference)))

(event EventTick
  (params (DeltaSeconds :type Float%20%28single-precision%29))
  (CallFunction|GetKeypointsLocations))

(fn ConstructionScript)

(fn GetKeypointsLocations
  (for (_array_element _array_index) (Variables|Default|GetKeypointsNames)
    (Utilities|Array|SetArrayElem (Variables|Default|GetKeypointsLoc) _array_index (Transformation|GetSocketLocation (Variables|Default|GetFaceSkeletal) _array_element) true)))