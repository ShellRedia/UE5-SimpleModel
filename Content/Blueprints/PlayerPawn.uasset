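; Player pawn for a MetaHuman viewer that shows the main UI widget with a mouse cursor and provides viewport camera controls.
; On BeginPlay it caches the first actor of the selected MetaHuman class.
; ViewportMove dispatches to vertical, horizontal or distance moves, each returning a position or running count.
; Horizontal moves also shift depth to approximate an arc, then re-aim the camera at the MetaHuman at camera height, keeping it level.
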(event EventBeginPlay
  (Utilities|FlowControl|Sequence
    (:then_0
      (bind _returnvalue (UserInterface|CreateWidget "/Game/UI/WidgetMain.WidgetMain_C"))
      (UserInterface|Viewport|AddtoViewport _returnvalue 0)
      (Variables|/Script/Engine.PlayerController|SetbShowMouseCursor (Game|GetPlayerController 0) true))
    (:then_1
      (bind _outactors (Actor|GetAllActorsOfClass (Utilities|Array|Get(acopy) (Variables|Default|GetMetaHumanClasses) (Variables|Default|GetMetaHumanIndex))))
      (Variables|Default|SetMetaHumanRef (Utilities|Array|Get(acopy) _outactors)))))

(event Collision|EventActorBeginOverlap
  (params (OtherActor :type Actor%20Object%20Reference)))

(event EventTick
  (params (DeltaSeconds :type Float%20%28single-precision%29)))

(fn ConstructionScript)

(fn ViewportMove
  (params (MoveAxis :type String) (Delta :type Integer))
  (switch string MoveAxis
    (:Vertical
      (bind _currentvalue (CallFunction|MoveVertical Delta))
      (return _currentvalue))
    (:Horizontal
      (bind _currentvalue_2 (CallFunction|MoveHorizontal Delta))
      (return _currentvalue_2))
    (:Distance
      (bind _currentvalue_3 (CallFunction|MoveDistance Delta))
      (return _currentvalue_3))))

(fn MoveVertical
  (params (Delta :type Integer))
  (bind _camera (Variables|Default|GetCamera))
  (Transformation|AddLocalOffset _camera (Math|Vector|MakeVector 0.0 0.0 (Math|Conversions|ToFloat(Integer) Delta)) false false)
  (return (Math|Float|Truncate (.z (Variables|/Script/Engine.SceneComponent|GetRelativeLocation _camera)))))

(fn MoveHorizontal
  (params (Delta :type Integer))
  (bind _returnvalue (Math|Conversions|ToFloat(Integer) Delta))
  (bind _camera (Variables|Default|GetCamera))
  (bind _camera_2 (Variables|Default|GetCamera))
  (bind _metahumanref (Variables|Default|GetMetaHumanRef))
  (bind _returnvalue_2 (Transformation|GetActorLocation _metahumanref))
  (bind _returnvalue_3 (Math|Float|Absolute(Float) _returnvalue))
  (bind _relativelocation (Variables|/Script/Engine.SceneComponent|GetRelativeLocation _camera_2))
  (Utilities|IsValid (Variables|Default|GetMetaHumanRef)
    (:Is%20Valid
      (if (> (* _returnvalue (.y _relativelocation)) 0.5)
        (Transformation|AddRelativeLocation _camera (Math|Vector|MakeVector _returnvalue_3 _returnvalue 0.0) false false)
        (else
          (Transformation|AddRelativeLocation (Variables|Default|GetCamera) (Math|Vector|MakeVector (* _returnvalue_3 -1.0) _returnvalue 0.0) false false)))
      (Transformation|SetWorldRotation _camera (Math|Rotator|FindLookatRotation (Transformation|GetWorldLocation _camera_2) (Math|Vector|MakeVector (.x _returnvalue_2) (.y _returnvalue_2) (.z (Transformation|GetWorldLocation _camera_2)))) false false)
      (return (Math|Float|Truncate (.y _relativelocation))))))

(fn MoveDistance
  (params (Delta :type Integer))
  (Variables|Default|SetDistanceCount (+ Delta (Variables|Default|GetDistanceCount)))
  (bind _result (Utilities|NegateInt Delta)
    (:%20%20
      (Transformation|AddLocalOffset (Variables|Default|GetCamera) (Math|Vector|MakeVector (Math|Conversions|ToFloat(Integer) _result) 0.0 0.0) false false)
      (return (Variables|Default|GetDistanceCount)))))